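; Shared multiplayer camera that frames two to four players and becomes the view target for the player controllers.
; On BeginPlay it caches the player list from GameplayGM and starts a fast looping timer in place of Tick.
; Each update picks functions by player count, setting spring arm length to the largest pairwise player distance within min/max limits.
; The actor eases toward the players' average location with VInterpTo.
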(event Custom|UpdateCamera
  (switch int (Utilities|Array|Length (Variables|Default|GetPlayersReferance))
    (:2
      (CallFunction|SetArmLenghP2)
      (CallFunction|SetCameraPosP2))
    (:3
      (CallFunction|SetArmLenghP3)
      (CallFunction|SetCameraPosP3))
    (:4
      (CallFunction|SetArmLenghP4)
      (CallFunction|SetCameraPosP4))))

(event EventBeginPlay
  (CallFunction|ClassSetup)
  (Utilities|Time|SetTimerbyFunctionName 0 "UpdateCamera" 0.001 true))

(fn ConstructionScript)

(fn ClassSetup
  (bind _asgameplay_gm (Utilities|Casting|CastToGameplayGM (Game|GetGameMode)))
  (bind _output_get (Variables|Default|SetGameplayGM _asgameplay_gm))
  (Variables|Default|SetPlayersReferance (Variables|/Game/Blueprints/Gameplay/GameplayGM.GameplayGM_C|GetPlayers _output_get))
  (bind _outactors (Actor|GetAllActorsOfClass "/Script/Engine.PlayerController"))
  (Game|Player|SetViewTargetwithBlend _outactors self 0.0 "VTBlend_Linear" 0.0 false)
  (for (_array_element _array_index) (Variables|Default|GetPlayersReferance)
    (switch int _array_index
      (:0
        (Variables|Default|SetP1 _array_element))
      (:1
        (Variables|Default|SetP2 _array_element))
      (:2
        (Variables|Default|SetP3 _array_element))
      (:3
        (Variables|Default|SetP4 _array_element)))))

(fn SetArmLenghP4
  (bind _p1 (Variables|Default|GetP1))
  (bind _p2 (Variables|Default|GetP2))
  (bind _p3 (Variables|Default|GetP3))
  (bind _p4 (Variables|Default|GetP4))
  (Variables|/Script/Engine.SpringArmComponent|SetTargetArmLength (Variables|Default|GetSpringArm) (Math|Float|Clamp(Float) (.MaxValue (Math|Float|MaxOfFloatArray (Utilities|Array|MakeArray (Transformation|GetDistanceTo _p1 _p2) (Transformation|GetDistanceTo _p2 _p3) (Transformation|GetDistanceTo _p2 _p4) (Transformation|GetDistanceTo _p1 _p3) (Transformation|GetDistanceTo _p1 _p4) (Transformation|GetDistanceTo _p3 _p4)))) (Variables|Default|GetMinimumArmLengh) (Variables|Default|GetMaximumArmLengh))))

(fn SetArmLenghP3
  (bind _p1 (Variables|Default|GetP1))
  (bind _p2 (Variables|Default|GetP2))
  (bind _p3 (Variables|Default|GetP3))
  (Variables|/Script/Engine.SpringArmComponent|SetTargetArmLength (Variables|Default|GetSpringArm) (Math|Float|Clamp(Float) (.MaxValue (Math|Float|MaxOfFloatArray (Utilities|Array|MakeArray (Transformation|GetDistanceTo _p1 _p2) (Transformation|GetDistanceTo _p2 _p3) (Transformation|GetDistanceTo _p1 _p3)))) (Variables|Default|GetMinimumArmLengh) (Variables|Default|GetMaximumArmLengh))))

(fn SetArmLenghP2
  (Variables|/Script/Engine.SpringArmComponent|SetTargetArmLength (Variables|Default|GetSpringArm) (Math|Float|Clamp(Float) (Transformation|GetDistanceTo (Variables|Default|GetP1) (Variables|Default|GetP2)) (Variables|Default|GetMinimumArmLengh) (Variables|Default|GetMaximumArmLengh))))

(fn SetCameraPosP4
  (Variables|Default|SetTargetPos (/ (+ (Transformation|GetActorLocation (Variables|Default|GetP1)) (Transformation|GetActorLocation (Variables|Default|GetP2)) (Transformation|GetActorLocation (Variables|Default|GetP3)) (Transformation|GetActorLocation (Variables|Default|GetP4))) (Math|Conversions|ToFloat(Integer) (Utilities|Array|Length (Variables|Default|GetPlayersReferance)))))
  (Transformation|SetActorLocation (Math|Interpolation|VInterpTo (Variables|Default|GetPreviousPos) (Variables|Default|GetTargetPos) (Utilities|Time|GetWorldDeltaSeconds) (Variables|Default|GetInterpSpeed)) false false)
  (Variables|Default|SetPreviousPos (Transformation|GetActorLocation)))

(fn SetCameraPosP3
  (Variables|Default|SetTargetPos (/ (+ (Transformation|GetActorLocation (Variables|Default|GetP1)) (Transformation|GetActorLocation (Variables|Default|GetP2)) (Transformation|GetActorLocation (Variables|Default|GetP3))) (Math|Conversions|ToFloat(Integer) (Utilities|Array|Length (Variables|Default|GetPlayersReferance)))))
  (Transformation|SetActorLocation (Math|Interpolation|VInterpTo (Variables|Default|GetPreviousPos) (Variables|Default|GetTargetPos) (Utilities|Time|GetWorldDeltaSeconds) (Variables|Default|GetInterpSpeed)) false false)
  (Variables|Default|SetPreviousPos (Transformation|GetActorLocation)))

(fn SetCameraPosP2
  (Variables|Default|SetTargetPos (/ (+ (Transformation|GetActorLocation (Variables|Default|GetP1)) (Transformation|GetActorLocation (Variables|Default|GetP2))) (Math|Conversions|ToFloat(Integer) (Utilities|Array|Length (Variables|Default|GetPlayersReferance)))))
  (Transformation|SetActorLocation (Math|Interpolation|VInterpTo (Variables|Default|GetPreviousPos) (Variables|Default|GetTargetPos) (Utilities|Time|GetWorldDeltaSeconds) (Variables|Default|GetInterpSpeed)) false false)
  (Variables|Default|SetPreviousPos (Transformation|GetActorLocation)))