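; BP_ProjectionCharacter is a short-lived, AI-moved projection character from the power-up Blueprints that wanders the level.
; On BeginPlay it starts a roaming loop using AI MoveTo toward random navigable points within a radius of its current location.
; Both success and failure retrigger the move after a short delay.
; A separate delay after the first move request destroys the actor after ten seconds.
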(event Custom|MoveToRandomLocation
  (AI|AIMoveTo self (Class|NavigationSystem|GetRandomPointinNavigableRadius (Transformation|GetActorLocation) 2.5e+03) 0 5.0 false
    (:OnSuccess
      (Utilities|FlowControl|Delay 1.0)
      (CallFunction|MovetoRandomLocation))
    (:OnFail
      (Utilities|FlowControl|Delay 1.0)
      (CallFunction|MovetoRandomLocation))))

(event EventBeginPlay
  (CallFunction|MovetoRandomLocation)
  (Utilities|FlowControl|Delay 1e+01)
  (Actor|DestroyActor))

(fn ConstructionScript)